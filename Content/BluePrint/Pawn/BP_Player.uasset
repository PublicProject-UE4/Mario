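; Player character for a Mario-style 2D side-scroller, with movement, crouching, fireballs, star invincibility, damage, death and a flagpole finish.
; The power-up tier (Mini, Big, Fire) lives in BP_GameInstance and selects capsule size, flipbook set and abilities.
; Movement input drives state, animation, facing and power-up updates; Tick takes these over after finishing and runs the camera and countdown.
; Also includes debug keys for level loading and collision display.
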(event OnComponentBeginOverlap(Box_Top)
  (params (OverlappedComponent :type Primitive%20Component%20Object%20Reference) (OtherActor :type Actor%20Object%20Reference) (OtherComp :type Primitive%20Component%20Object%20Reference) (OtherBodyIndex :type Integer) (bFromSweep :type Boolean) (SweepResult :type Hit%20Result%20Structure%20%28by%20ref%29))
  ;[1 1 1] CrouchLock
  (Variables|Default|SetbCrouchLock true))

(event OnComponentEndOverlap(Box_Top)
  (params (OverlappedComponent :type Primitive%20Component%20Object%20Reference) (OtherActor :type Actor%20Object%20Reference) (OtherComp :type Primitive%20Component%20Object%20Reference) (OtherBodyIndex :type Integer))
  ;[1 1 1] CrouchLock
  (Variables|Default|SetbCrouchLock false))

(event OnComponentBeginOverlap(Box_Star)
  (params (OverlappedComponent :type Primitive%20Component%20Object%20Reference) (OtherActor :type Actor%20Object%20Reference) (OtherComp :type Primitive%20Component%20Object%20Reference) (OtherBodyIndex :type Integer) (bFromSweep :type Boolean) (SweepResult :type Hit%20Result%20Structure%20%28by%20ref%29))
  ;[1 1 1] Power UP
  (if (Variables|Anim|GetbStar)
    (Game|Damage|ApplyDamage OtherActor 1.0 0 0)))

(event Custom|LoadGame
  (bind _returnvalue (Game|GetGameInstance))
  (bind _asbp_game_instance (Utilities|Casting|CastToBP_GameInstance _returnvalue))
  (bind _restartpos (Variables|/Game/BluePrint/BP_GameInstance.BP_GameInstance_C|GetReStartPos _asbp_game_instance))
  ;[1 1 1] LoadGame,读取游戏
  (if (Math|Vector|NotEqual(Vector) "0, 0, 0" _restartpos 0.0001)
    (Transformation|SetActorLocation _restartpos false false)))

(event Custom|CameraZ
  (bind _returnvalue (Transformation|GetActorLocation))
  ;[1 1 1] Tick_CameraZ
  (Transformation|SetWorldLocation (Variables|Default|GetSpringArm) (Math|Vector|MakeVector (.x _returnvalue) (.y _returnvalue) 0.0) false false))

(event Custom|StarMode
  ;[1 1 1] Power UP
  (Variables|Default|SetbInvincible true)
  (Rendering|Material|SetMaterial (Variables|Default|GetSprite) 0 "/Game/Art/Material/Star.Star")
  (Collision|SetCollisionEnabled (Variables|Default|GetBox_Star) "QueryOnly")
  (Utilities|FlowControl|Delay (Variables|Time|GetStarTime))
  (Collision|SetCollisionEnabled (Variables|Default|GetBox_Star) "QueryOnly")
  (Rendering|Material|SetMaterial (Variables|Default|GetSprite) 0 0)
  (Variables|Anim|SetbStar false)
  (Variables|Default|SetbInvincible false))

(event Custom|Finish
  ;[1 1 1] Goal
  (if (Variables|Goal|GetbFinish)
    (CallFunction|MoveSetup)
    (CallFunction|UpdataAnim)
    (CallFunction|PowerUp)
    (CallFunction|FlipSprite)
    (CallFunction|GoalScean)))

(event Custom|CountDownTimer
  (bind _returnvalue (Game|GetGameInstance))
  (bind _asbp_game_instance (Utilities|Casting|CastToBP_GameInstance _returnvalue))
  ;[1 1 1] CountDownTimer
  (if (Variables|Goal|GetbFinish)
    (if (Variables|Goal|GetbFinishCastle)
      (if (!= 0 (Variables|Time|GetCountDown))
        (Variables|Time|SetCountDown (- (Variables|Time|GetCountDown) 1))
        (Variables|/Game/BluePrint/BP_GameInstance.BP_GameInstance_C|SetPointCount _asbp_game_instance (+ 50 (Variables|/Game/BluePrint/BP_GameInstance.BP_GameInstance_C|GetPointCount _asbp_game_instance)))
        (if (!= 0 (Variables|Time|GetCountDown))
          (Utilities|FlowControl|DoOnce false :!label _label
            (:Completed
              (Audio|PlaySound2D "/Game/Sound/SE/SE_Count3.SE_Count3" 1.0 1.0 0.0 0 0)
              (Utilities|FlowControl|Delay 0.05)
              (goto _label Reset))))))
    (elif (not (Variables|Anim|GetbDeath))
      (bind _output_get (Variables|Time|SetTime (+ (Utilities|Time|GetWorldDeltaSeconds) (Variables|Time|GetTime))))
      (Variables|Time|SetCountDown (- 400 (Math|Float|Truncate _output_get)))
      (if (== 0 (Variables|Time|GetCountDown))
        (CallFunction|TimeDeath)))))

(event Custom|MoveSetup
  ;[1 1 1] MoveSetup
  (Variables|Anim|SetbMoving (!= (Math|Vector|VectorLength (Transformation|GetVelocity)) 0.0))
  (Variables|Anim|SetbFalling (AI|Components|NavMovement|IsFalling (Variables|Character|GetCharacterMovement)))
  (Variables|Anim|SetbBraking (> -5e+01 (* (Input|AxisValues|GetMoveRight) (.x (Transformation|GetVelocity))))))

(event Custom|UpdataAnim
  ;[1 1 1] UpdataAnim(更新角色动画)
  (switch Utilities|FlowControl|Switch|SwitchonPowerUp (Variables|/Game/BluePrint/BP_GameInstance.BP_GameInstance_C|GetPowerUp (.AsBP%20Game%20Instance (Utilities|Casting|CastToBP_GameInstance (Game|GetGameInstance))))
    (:NewEnumerator0
      (CallFunction|AnimMini))
    (:NewEnumerator1
      (CallFunction|AnimBig))
    (:NewEnumerator2
      (CallFunction|AnimFire))))

(event Custom|PowerUp
  ;[1 1 1] Power UP
  (if (Variables|Anim|GetbStar)
    (CallFunction|StarMode))
  (Utilities|FlowControl|Sequence
    (:then_0
      (switch Utilities|FlowControl|Switch|SwitchonPowerUp (Variables|/Game/BluePrint/BP_GameInstance.BP_GameInstance_C|GetPowerUp (.AsBP%20Game%20Instance (Utilities|Casting|CastToBP_GameInstance (Game|GetGameInstance))))
        (:NewEnumerator0
          (Components|Capsule|SetCapsuleHalfHeight (Variables|Collision|GetCapsuleComponent) 6.0 true))))
    (:then_1
      (if (Variables|Anim|GetbPowerUp_Big)
        (Variables|Default|SetbInvincible true)
        (Components|Capsule|SetCapsuleHalfHeight (Variables|Collision|GetCapsuleComponent) 14.0 true)
        (Input|DisableInput 0)
        (Utilities|FlowControl|Delay 0.5)
        (Input|EnableInput 0)
        (Variables|Anim|SetbPowerUp_Big false)
        (Variables|/Game/BluePrint/BP_GameInstance.BP_GameInstance_C|SetPowerUp (.AsBP%20Game%20Instance (Utilities|Casting|CastToBP_GameInstance (Game|GetGameInstance))) "NewEnumerator1")
        (Utilities|FlowControl|Delay 0.5)
        (Variables|Default|SetbInvincible false)
        (elif (Variables|Anim|GetbPowerUp_Fire)
          (Variables|Default|SetbInvincible true)
          (Components|Capsule|SetCapsuleHalfHeight (Variables|Collision|GetCapsuleComponent) 14.0 true)
          (Input|DisableInput 0)
          (Utilities|FlowControl|Delay 0.5)
          (Input|EnableInput 0)
          (Variables|Anim|SetbPowerUp_Fire false)
          (Variables|/Game/BluePrint/BP_GameInstance.BP_GameInstance_C|SetPowerUp (.AsBP%20Game%20Instance (Utilities|Casting|CastToBP_GameInstance (Game|GetGameInstance))) "NewEnumerator2")
          (Utilities|FlowControl|Delay 0.5)
          (Variables|Default|SetbInvincible false)
          (elif (Variables|Anim|GetbDamage)
            (Variables|Default|SetbInvincible true)
            (Components|Capsule|SetCapsuleHalfHeight (Variables|Collision|GetCapsuleComponent) 14.0 true)
            (Utilities|FlowControl|Delay 0.5)
            (Variables|Anim|SetbDamage false)
            (Variables|/Game/BluePrint/BP_GameInstance.BP_GameInstance_C|SetPowerUp (.AsBP%20Game%20Instance (Utilities|Casting|CastToBP_GameInstance (Game|GetGameInstance))) "NewEnumerator0")
            (Utilities|FlowControl|Delay 0.5)
            (Variables|Default|SetbInvincible false)))))))

(event Custom|FlipSprite
  ;[1 1 1] FlipSprite(设置角色的翻转)
  (if (not (Variables|Anim|GetbFalling))
    (Math|Float|CompareFloat (Input|AxisValues|GetMoveRight) 0.0
      (:>
        (Pawn|SetControlRotation (Game|GetPlayerController 0) (Math|Rotator|MakeRotator 0.0 0.0 0.0)))
      (:<
        (Pawn|SetControlRotation (Game|GetPlayerController 0) (Math|Rotator|MakeRotator 0.0 0.0 1.8e+02))))))

(event Custom|GoalScean
  (bind _charactermovement (Variables|Character|GetCharacterMovement))
  ;[1 1 1] Goal
  (if (Variables|Anim|GetbGoal)
    (Utilities|FlowControl|DoOnce false
      (:Completed
        (Variables|/Script/Engine.CharacterMovementComponent|SetGravityScale _charactermovement 0.0)
        (Components|Movement|StopMovementImmediately _charactermovement)
        (Input|DisableInput 0)
        (bind _alpha (Timeline|Timeline_FlagDown Play)
          (:Update
            (Transformation|SetActorLocation (Math|Vector|Lerp(Vector) (Variables|Goal|GetGoalHeight) (Variables|Goal|GetGoalDown_Pos) _alpha) false false))
          (:Finished
            (Utilities|FlowControl|Delay 0.2)
            (Transformation|SetActorLocation (Variables|Goal|GetGoalDownRight_Pos) false false)
            (Pawn|SetControlRotation (Game|GetPlayerController 0) (Math|Rotator|MakeRotator 0.0 0.0 1.8e+02))
            (Utilities|FlowControl|Delay 1.0)
            (Variables|/Script/Engine.CharacterMovementComponent|SetGravityScale (Variables|Character|GetCharacterMovement) 1.0)
            (Variables|Anim|SetbGoal false)))))
    (else
      (Pawn|Input|AddMovementInput "1.000000, 0, 0" (Variables|Goal|GetFinish_Walk) false)
      (if (Variables|Goal|GetbFinishCastle)
        (Pawn|Components|CharacterMovement|DisableMovement (Variables|Character|GetCharacterMovement))
        (Rendering|SetActorHiddenInGame true)
        (if (== 0 (Variables|Time|GetCountDown))
          (Utilities|FlowControl|Delay 1.0)
          (Game|OpenLevel(byName) "01Select"))))))

(event Custom|TimeDeath
  ;[1 1 1] Damage(受到伤害时的一些相应的变化)
  (Utilities|FlowControl|Sequence
    (:then_0
      (Variables|Anim|SetbDeath true)
      (Pawn|Components|CharacterMovement|DisableMovement (Variables|Character|GetCharacterMovement))
      (Collision|SetActorEnableCollision false)
      (bind _asbp_game_instance (Utilities|Casting|CastToBP_GameInstance (Game|GetGameInstance)))
      (Default|Death _asbp_game_instance))
    (:then_1
      (Utilities|FlowControl|Delay 1.0)
      (Rendering|SetActorHiddenInGame true)
      (Input|DisableInput 0)
      (bind _returnvalue (Game|SpawnActorfromClass "/Game/BluePrint/Object/Spawn/BP_Player_Death.BP_Player_Death_C" (Transformation|GetActorTransform) "Undefined" 0 0))
      ;;[1 1 1] 向上的一个能量，人物死后向上冲击的力
      (Physics|AddImpulse (Variables|/Game/BluePrint/Object/Spawn/BP_Player_Death.BP_Player_Death_C|GetPaperSprite _returnvalue) "0, 0,512.000000" "None" false))
    (:then_2
      (Utilities|FlowControl|Delay 3.0)
      (Game|OpenLevel(byName) "01Select"))))

(event EventBeginPlay
  ;[0 1 0] BeginPlay
  (Class|ActorComponent|SetIsReplicated (Variables|Default|GetSprite) true)
  (bind _returnvalue (UserInterface|CreateWidget "/Game/BluePrint/HUD/BP_Player_HUD.BP_Player_HUD_C"))
  (UserInterface|Viewport|AddtoViewport _returnvalue 0)
  (Variables|/Script/Engine.PlayerController|SetbShowMouseCursor (Game|GetPlayerController 0) true)
  (CallFunction|LoadGame)
  (Collision|SetCollisionEnabled (Variables|Default|GetBox_Star) "NoCollision"))

(event Game|Damage|EventAnyDamage
  (params (Damage :type Float%20%28single-precision%29) (DamageType :type Damage%20Type%20Object%20Reference) (InstigatedBy :type Controller%20Object%20Reference) (DamageCauser :type Actor%20Object%20Reference))
  (bind _returnvalue (Game|GetGameInstance))
  (bind _asbp_game_instance (Utilities|Casting|CastToBP_GameInstance _returnvalue))
  ;[1 1 1] Damage(受到伤害时的一些相应的变化)
  (if (not (Variables|Default|GetbInvincible))
    (switch Utilities|FlowControl|Switch|SwitchonPowerUp (Variables|/Game/BluePrint/BP_GameInstance.BP_GameInstance_C|GetPowerUp _asbp_game_instance)
      (:NewEnumerator0
        (Utilities|FlowControl|Sequence
          (:then_0
            (Variables|Anim|SetbDeath true)
            (Pawn|Components|CharacterMovement|DisableMovement (Variables|Character|GetCharacterMovement))
            (Collision|SetActorEnableCollision false)
            (bind _asbp_game_instance_2 (Utilities|Casting|CastToBP_GameInstance (Game|GetGameInstance)))
            (Default|Death _asbp_game_instance_2))
          (:then_1
            (Utilities|FlowControl|Delay 1.0)
            (Rendering|SetActorHiddenInGame true)
            (Input|DisableInput 0)
            (bind _returnvalue_2 (Game|SpawnActorfromClass "/Game/BluePrint/Object/Spawn/BP_Player_Death.BP_Player_Death_C" (Transformation|GetActorTransform) "Undefined" 0 0))
            ;;[1 1 1] 向上的一个能量，人物死后向上冲击的力
            (Physics|AddImpulse (Variables|/Game/BluePrint/Object/Spawn/BP_Player_Death.BP_Player_Death_C|GetPaperSprite _returnvalue_2) "0, 0,512.000000" "None" false))
          (:then_2
            (Utilities|FlowControl|Delay 3.0)
            (Game|OpenLevel(byName) "01Select"))))
      (:NewEnumerator1
        (Variables|/Game/BluePrint/BP_GameInstance.BP_GameInstance_C|SetPowerUp _asbp_game_instance "NewEnumerator1" :!label _label)
        (Variables|Anim|SetbDamage true)
        (Utilities|SoundEffect) ; enters at Damage
      )
      (:NewEnumerator2
        (goto _label)))))

(event EventTick
  (params (DeltaSeconds :type Float%20%28single-precision%29))
  ;[1 0.5 0.5] Tick
  (CallFunction|CameraZ)
  (CallFunction|Finish)
  (CallFunction|CountDownTimer))

(event Input|ActionEvents|InputActionJump
  (params (Key :type Key%20Structure :default "None"))
  ;[1 1 1] Jump(跳)
  (:Pressed
    (if (Variables|Anim|GetbCrouching)
      (if (not (Variables|Anim|GetbFalling))
        (Character|LaunchCharacter "0, 0,300.000000" false false)
        (Utilities|SoundEffect :!label _label) ; enters at Jump
      )
      (else
        (Character|Jump)
        (goto _label Jump))))
  (:Released
    (Character|StopJumping)))

(event Input|ActionEvents|InputActionDash
  (params (Key :type Key%20Structure :default "None"))
  (bind _charactermovement (Variables|Character|GetCharacterMovement))
  ;[1 1 1] Dash
  (:Pressed
    (Variables|/Script/Engine.CharacterMovementComponent|SetMaxWalkSpeed _charactermovement 1.5e+02))
  (:Released
    (Variables|/Script/Engine.CharacterMovementComponent|SetMaxWalkSpeed _charactermovement 8e+01)))

(event Input|ActionEvents|InputActionFireball
  (params (Key :type Key%20Structure :default "None"))
  ;[1 1 1] Fireball(发射子弹)
  (:Pressed
    (switch Utilities|FlowControl|Switch|SwitchonPowerUp (Variables|/Game/BluePrint/BP_GameInstance.BP_GameInstance_C|GetPowerUp (.AsBP%20Game%20Instance (Utilities|Casting|CastToBP_GameInstance (Game|GetGameInstance))))
      (:NewEnumerator2
        (Utilities|FlowControl|DoN 2 :!label _label
          (:Exit
            (Utilities|FlowControl|Sequence
              (:then_0
                (Variables|Anim|SetbFire_Attack true)
                (bind _returnvalue (Game|SpawnActorfromClass "/Game/BluePrint/Object/Spawn/BP_Fireball.BP_Fireball_C" (Transformation|GetWorldTransform (Variables|Default|GetFireball_Spawn_Pos)) "Undefined" 0 0))
                (Pawn|SpawnDefaultController _returnvalue)
                (Character|LaunchCharacter _returnvalue (Math|Vector|MakeVector (* (.x (Transformation|GetActorForwardVector)) 2e+02) 0.0 -5e+01) false false)
                (Utilities|SoundEffect))
              (:then_1
                (Character|UnCrouch)
                (Utilities|FlowControl|Delay 0.5)
                (Variables|Anim|SetbFire_Attack false)
                (Utilities|FlowControl|Delay 0.5)
                (goto _label Reset))))))))
  (:Released
    (Variables|Anim|SetbFire_Attack false)))

(event Input|ActionEvents|InputActionPause
  (params (Key :type Key%20Structure :default "None"))
  ;[1 1 1] 2020年7月27日16:23:19 按键事件
  (:Pressed
    (if (Game|IsGamePaused)
      (Game|SetGamePaused false)
      (Utilities|SoundEffect :!label _label) ; enters at Pause
      (else
        (Game|SetGamePaused true)
        (goto _label Pause)))))

(event Input|ActionEvents|InputActionQuit
  (params (Key :type Key%20Structure :default "None"))
  ;[1 1 1] 2020年7月27日16:23:19 按键事件
  (:Pressed
    (Game|QuitGame 0 "Quit" false)))

(event Input|AxisEvents|InputAxisMoveRight
  (params (AxisValue :type Float%20%28single-precision%29))
  ;[1 1 1] MoveRight
  (Pawn|Input|AddMovementInput "0, 0, 0" AxisValue false)
  (CallFunction|MoveSetup)
  (CallFunction|UpdataAnim)
  (CallFunction|PowerUp)
  (CallFunction|FlipSprite)
  (CallFunction|StopJump)
  (CallFunction|WarpTrigger)
  (Utilities|SoundEffect) ; enters at Brake
)

(event Input|AxisEvents|InputAxisMoveUp
  (params (AxisValue :type Float%20%28single-precision%29))
  ;[1 1 1] Move Up
  (if (< AxisValue 0.0)
    (Collision|SetCollisionEnabled (Variables|Default|GetBox_Bottom) "QueryOnly")
    (else
      (Collision|SetCollisionEnabled (Variables|Default|GetBox_Bottom) "NoCollision")))
  (switch Utilities|FlowControl|Switch|SwitchonPowerUp (Variables|/Game/BluePrint/BP_GameInstance.BP_GameInstance_C|GetPowerUp (.AsBP%20Game%20Instance (Utilities|Casting|CastToBP_GameInstance (Game|GetGameInstance))))
    (:NewEnumerator0
      (Character|UnCrouch))
    (:NewEnumerator1
      (if (Variables|Default|GetbCrouchLock) :!label _label
        (Character|Crouch)
        (else
          (bind _output_get (Variables|Anim|SetbCrouching (< (Input|AxisValues|GetMoveUp) 0.0)))
          (if _output_get
            (if (Variables|Anim|GetbFire_Attack)
              (Character|UnCrouch)
              (else
                (Character|Crouch)))
            (else
              (Character|UnCrouch))))))
    (:NewEnumerator2
      (goto _label))))

(event Input|KeyboardEvents|R
  (params (Key :type Key%20Structure :default "None"))
  ;[1 1 1] 2020年7月27日16:23:19 按键事件
  (:Pressed
    (Development|ExecuteConsoleCommand "ReStartLevel" 0)))

(event Input|KeyboardEvents|C
  (params (Key :type Key%20Structure :default "None"))
  ;[1 1 1] 2020年7月27日16:23:19 按键事件
  (:Pressed
    (Development|ExecuteConsoleCommand "Show Collision" 0)))

(event Input|KeyboardEvents|0
  (params (Key :type Key%20Structure :default "None"))
  ;[1 1 1] 2020年7月27日16:23:19 按键事件
  (:Pressed
    (Game|OpenLevel(byName) "10Test")))

(event Input|KeyboardEvents|1
  (params (Key :type Key%20Structure :default "None"))
  ;[1 1 1] 2020年7月27日16:23:19 按键事件
  (:Pressed
    (Game|OpenLevel(byName) "00Start")))

(event Input|KeyboardEvents|2
  (params (Key :type Key%20Structure :default "None"))
  ;[1 1 1] 2020年7月27日16:23:19 按键事件
  (:Pressed
    (Game|OpenLevel(byName) "11Level")))

(event Input|KeyboardEvents|3
  (params (Key :type Key%20Structure :default "None"))
  ;[1 1 1] 2020年7月27日16:23:19 按键事件
  (:Pressed
    (Game|OpenLevel(byName) "12Level")))

(fn ConstructionScript)

(fn AnimMini
  (if (Variables|Anim|GetbGoal)
    (LocalVariables|SetAnimStateMini "NewEnumerator5")
    (elif (Variables|Anim|GetbDeath)
      (LocalVariables|SetAnimStateMini "NewEnumerator4")
      (elif (Variables|Anim|GetbFalling)
        (LocalVariables|SetAnimStateMini "NewEnumerator2")
        (elif (Variables|Anim|GetbBraking)
          (LocalVariables|SetAnimStateMini "NewEnumerator3")
          (elif (Variables|Anim|GetbMoving)
            (LocalVariables|SetAnimStateMini "NewEnumerator1")
            (else
              (LocalVariables|SetAnimStateMini "NewEnumerator0")))))))
  (Sprite|SetFlipbook (Variables|Default|GetSprite) (Utilities|Select :Index (LocalVariables|GetAnimStateMini) :NewEnumerator0 "/Game/Art/Sprite/00_mini_idle.00_mini_idle" :NewEnumerator1 "/Game/Art/Sprite/00_mini_walk.00_mini_walk" :NewEnumerator2 "/Game/Art/Sprite/00_mini_jump.00_mini_jump" :NewEnumerator3 "/Game/Art/Sprite/00_mini_brake.00_mini_brake" :NewEnumerator4 "/Game/Art/Sprite/00_mini_death.00_mini_death" :NewEnumerator5 "/Game/Art/Sprite/00_mini_goal.00_mini_goal")))

(fn AnimBig
  (if (Variables|Anim|GetbGoal)
    (LocalVariables|SetAnimStateBig "NewEnumerator8")
    (elif (Variables|Anim|GetbPowerUp_Big)
      (LocalVariables|SetAnimStateBig "NewEnumerator5")
      (elif (Variables|Anim|GetbPowerUp_Fire)
        (LocalVariables|SetAnimStateBig "NewEnumerator6")
        (elif (Variables|Anim|GetbDamage)
          (LocalVariables|SetAnimStateBig "NewEnumerator7")
          (elif (Variables|Anim|GetbCrouching)
            (LocalVariables|SetAnimStateBig "NewEnumerator4")
            (elif (Variables|Anim|GetbFalling)
              (LocalVariables|SetAnimStateBig "NewEnumerator2")
              (elif (Variables|Anim|GetbBraking)
                (LocalVariables|SetAnimStateBig "NewEnumerator3")
                (elif (Variables|Anim|GetbMoving)
                  (LocalVariables|SetAnimStateBig "NewEnumerator1")
                  (else
                    (LocalVariables|SetAnimStateBig "NewEnumerator0"))))))))))
  (Sprite|SetFlipbook (Variables|Default|GetSprite) (Utilities|Select :Index (LocalVariables|GetAnimStateBig) :NewEnumerator0 "/Game/Art/Sprite/01_player_idle.01_player_idle" :NewEnumerator1 "/Game/Art/Sprite/01_player_walk.01_player_walk" :NewEnumerator2 "/Game/Art/Sprite/01_player_jump.01_player_jump" :NewEnumerator3 "/Game/Art/Sprite/01_player_brake.01_player_brake" :NewEnumerator4 "/Game/Art/Sprite/01_player_crouch.01_player_crouch" :NewEnumerator5 "/Game/Art/Sprite/01_player_PUBig.01_player_PUBig" :NewEnumerator6 "/Game/Art/Sprite/01_player_PUFire.01_player_PUFire" :NewEnumerator7 "/Game/Art/Sprite/01_player_damage.01_player_damage" :NewEnumerator8 "/Game/Art/Sprite/01_player_goal.01_player_goal")))

(fn AnimFire
  (if (Variables|Anim|GetbGoal)
    (LocalVariables|SetAnimStateFire "NewEnumerator6")
    (elif (Variables|Anim|GetbFire_Attack)
      (LocalVariables|SetAnimStateFire "NewEnumerator5")
      (elif (Variables|Anim|GetbCrouching)
        (LocalVariables|SetAnimStateFire "NewEnumerator4")
        (elif (Variables|Anim|GetbFalling)
          (LocalVariables|SetAnimStateFire "NewEnumerator2")
          (elif (Variables|Anim|GetbBraking)
            (LocalVariables|SetAnimStateFire "NewEnumerator3")
            (elif (Variables|Anim|GetbMoving)
              (LocalVariables|SetAnimStateFire "NewEnumerator1")
              (else
                (LocalVariables|SetAnimStateFire "NewEnumerator0"))))))))
  (Sprite|SetFlipbook (Variables|Default|GetSprite) (Utilities|Select :Index (LocalVariables|GetAnimStateFire) :NewEnumerator0 "/Game/Art/Sprite/02_fire_idle.02_fire_idle" :NewEnumerator1 "/Game/Art/Sprite/02_fire_walk.02_fire_walk" :NewEnumerator2 "/Game/Art/Sprite/02_fire_jump.02_fire_jump" :NewEnumerator3 "/Game/Art/Sprite/02_fire_brake.02_fire_brake" :NewEnumerator4 "/Game/Art/Sprite/02_fire_crouch.02_fire_crouch" :NewEnumerator5 "/Game/Art/Sprite/02_fire_attack.02_fire_attack" :NewEnumerator6 "/Game/Art/Sprite/00_mini_goal.00_mini_goal")))

(fn StopJump
  (if (Variables|Anim|GetbFalling)
    (if (== 0.0 (.z (Transformation|GetVelocity)))
      (Character|StopJumping))))

(fn WarpTrigger
  (if (Variables|Anim|GetbFalling)
    (Collision|SetCollisionEnabled (Variables|Default|GetBox_Forward) "NoCollision")
    (elif (!= 0.0 (Input|AxisValues|GetMoveRight))
      (Collision|SetCollisionEnabled (Variables|Default|GetBox_Forward) "QueryOnly")
      (else
        (Collision|SetCollisionEnabled (Variables|Default|GetBox_Forward) "NoCollision")))))