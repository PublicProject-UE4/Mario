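; BP_Select is a level-transition Blueprint that shows a select HUD, then loads the map matching the game instance's Level index.
; On BeginPlay it calls LevelText on BP_GameInstance, adds BP_Select_HUD to the viewport and waits briefly before switching on Level to open a map by name.
; Shortcut keys jump directly to maps, restart the level or show collision, and input actions toggle pause with a sound or quit.
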(event EventBeginPlay
  (bind _returnvalue (Game|GetGameInstance))
  (bind _asbp_game_instance (Utilities|Casting|CastToBP_GameInstance _returnvalue))
  (Default|LevelText _asbp_game_instance)
  (bind _returnvalue_2 (UserInterface|CreateWidget "/Game/BluePrint/HUD/BP_Select_HUD.BP_Select_HUD_C"))
  (UserInterface|Viewport|AddtoViewport _returnvalue_2 0)
  (Utilities|FlowControl|Delay 3.0)
  (Development|PrintString "Level Map" true true "(R=1.000000,G=0.000000,B=0.000000,A=1.000000)" 1e+01)
  (switch int (Variables|/Game/BluePrint/BP_GameInstance.BP_GameInstance_C|GetLevel _asbp_game_instance)
    (:0
      (Game|OpenLevel(byName) "10Test"))
    (:1
      (Game|OpenLevel(byName) "00Start"))
    (:2
      (Game|OpenLevel(byName) "11Level"))
    (:3
      (Game|OpenLevel(byName) "12Level"))
    (:4
      (Game|OpenLevel(byName) "99GameOver"))))

(event Input|ActionEvents|InputActionPause
  (params (Key :type Key%20Structure :default "None"))
  ;[1 1 1] 2020年7月27日16:23:19 按键事件
  (:Pressed
    (if (Game|IsGamePaused)
      (Game|SetGamePaused false)
      (else
        (Game|SetGamePaused true)))
    (Audio|PlaySound2D "/Game/Sound/SE/SE_Pause.SE_Pause" 1.0 1.0 0.0 0 0)))

(event Input|ActionEvents|InputActionQuit
  (params (Key :type Key%20Structure :default "None"))
  ;[1 1 1] 2020年7月27日16:23:19 按键事件
  (:Pressed
    (Game|QuitGame 0 "Quit" false)))

(event Input|KeyboardEvents|R
  (params (Key :type Key%20Structure :default "None"))
  ;[1 1 1] 2020年7月27日16:23:19 按键事件
  (:Pressed
    (Development|ExecuteConsoleCommand "ReStartLevel" 0)))

(event Input|KeyboardEvents|C
  (params (Key :type Key%20Structure :default "None"))
  ;[1 1 1] 2020年7月27日16:23:19 按键事件
  (:Pressed
    (Development|ExecuteConsoleCommand "Show Collision" 0)))

(event Input|KeyboardEvents|0
  (params (Key :type Key%20Structure :default "None"))
  ;[1 1 1] 2020年7月27日16:23:19 按键事件
  (:Pressed
    (Game|OpenLevel(byName) "10Test")))

(event Input|KeyboardEvents|1
  (params (Key :type Key%20Structure :default "None"))
  ;[1 1 1] 2020年7月27日16:23:19 按键事件
  (:Pressed
    (Game|OpenLevel(byName) "00Start")))

(event Input|KeyboardEvents|2
  (params (Key :type Key%20Structure :default "None"))
  ;[1 1 1] 2020年7月27日16:23:19 按键事件
  (:Pressed
    (Game|OpenLevel(byName) "11Level")))

(event Input|KeyboardEvents|3
  (params (Key :type Key%20Structure :default "None"))
  ;[1 1 1] 2020年7月27日16:23:19 按键事件
  (:Pressed
    (Game|OpenLevel(byName) "12Level")))

(fn ConstructionScript)