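; BP_Camera_Pos is a placed camera zone that switches the first player's view to itself while BP_Player is inside its Box.
; Overlap begin blends to this actor; overlap end blends back to the player after a short delay, each with its own blend time.
; A delayed BeginPlay check snaps the view here if the player already starts inside.
; When CameraMove is set, Box_Move_Trigger plays a timeline that slides SceneComponent along local X.
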(event OnComponentBeginOverlap(Box)
  (params (OverlappedComponent :type Primitive%20Component%20Object%20Reference) (OtherActor :type Actor%20Object%20Reference) (OtherComp :type Primitive%20Component%20Object%20Reference) (OtherBodyIndex :type Integer) (bFromSweep :type Boolean) (SweepResult :type Hit%20Result%20Structure%20%28by%20ref%29))
  ;[1 1 1] 切换视角
  (Utilities|Casting|CastToBP_Player OtherActor)
  (Game|Player|SetViewTargetwithBlend (Game|GetPlayerController 0) self (Variables|Default|GetBeginBlendTime) "VTBlend_Linear" 0.0 false))

(event OnComponentEndOverlap(Box)
  (params (OverlappedComponent :type Primitive%20Component%20Object%20Reference) (OtherActor :type Actor%20Object%20Reference) (OtherComp :type Primitive%20Component%20Object%20Reference) (OtherBodyIndex :type Integer))
  ;[1 1 1] 切换视角
  (bind _asbp_player (Utilities|Casting|CastToBP_Player OtherActor))
  (if true
    (if true
      (Utilities|FlowControl|Delay 0.2)
      (Game|Player|SetViewTargetwithBlend (Game|GetPlayerController 0) _asbp_player (Variables|Default|GetEndBlendTime) "VTBlend_Linear" 0.0 false))))

(event OnComponentBeginOverlap(Box_Move_Trigger)
  (params (OverlappedComponent :type Primitive%20Component%20Object%20Reference) (OtherActor :type Actor%20Object%20Reference) (OtherComp :type Primitive%20Component%20Object%20Reference) (OtherBodyIndex :type Integer) (bFromSweep :type Boolean) (SweepResult :type Hit%20Result%20Structure%20%28by%20ref%29))
  (Utilities|Casting|CastToBP_Player OtherActor)
  (if (Variables|Default|GetCamera_Move)
    (bind _alpha (Timeline|Camera_Move_Timeline Play)
      (:Update
        (Transformation|SetRelativeLocation (Variables|Default|GetSceneComponent) (Math|Vector|Lerp(Vector) "0,300.000000, 0" "64.000000,300.000000, 0" _alpha) false false)))))

(event EventBeginPlay
  ;[1 1 1] BeginPlay
  (Utilities|FlowControl|Delay 0.2)
  (bind _asbp_player (Utilities|Casting|CastToBP_Player (Game|Player|GetPlayerPawn 0)))
  (if (Collision|IsOverlappingActor (Variables|Default|GetBox) _asbp_player :!class /Script/Engine.PrimitiveComponent)
    (Game|Player|SetViewTargetwithBlend (Game|GetPlayerController 0) self 0.0 "VTBlend_Linear" 0.0 false)))

(fn ConstructionScript)