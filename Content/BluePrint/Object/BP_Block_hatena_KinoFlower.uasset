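; Question block that gives the player a mushroom when Mini or a fire flower when Big or Fire, per the GameInstance PowerUp.
; A player overlapping the bottom box triggers it once: timelines bump the block and raise the item sprite in parallel.
; It then spawns a replacement block (class unset on the flower branch) and the pickup, destroying itself.
; The top box's launch/damage handler has its collision disabled from BeginPlay.
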(event OnComponentBeginOverlap(Box_Bottom)
  (params (OverlappedComponent :type Primitive%20Component%20Object%20Reference) (OtherActor :type Actor%20Object%20Reference) (OtherComp :type Primitive%20Component%20Object%20Reference) (OtherBodyIndex :type Integer) (bFromSweep :type Boolean) (SweepResult :type Hit%20Result%20Structure%20%28by%20ref%29))
  (Utilities|Casting|CastToBP_Player OtherActor)
  (Collision|SetCollisionEnabled (Variables|Default|GetBox_Bottom) "NoCollision")
  (Collision|SetCollisionEnabled (Variables|Default|GetBox_Top) "NoCollision")
  (Utilities|FlowControl|DoOnce false
    (:Completed
      (Audio|PlaySound2D "/Game/Sound/SE/SE_ItemSpawn.SE_ItemSpawn" 1.0 1.0 0.0 0 0)
      (switch Utilities|FlowControl|Switch|SwitchonPowerUp (Variables|/Game/BluePrint/BP_GameInstance.BP_GameInstance_C|GetPowerUp (.AsBP%20Game%20Instance (Utilities|Casting|CastToBP_GameInstance (Game|GetGameInstance))))
        (:NewEnumerator0
          ;[1 1 1] kinoko
          (Utilities|FlowControl|Sequence
            (:then_0
              (bind _alpha (Timeline|BlockUp Play)
                (:Update
                  (Transformation|SetRelativeLocation (Variables|Default|GetBox_Collision) (Math|Vector|Lerp(Vector) "0, 0, 0" "0, 0,4.000000" _alpha) false false))
                (:Finished
                  (bind _alpha_2 (Timeline|BlockDown Play)
                    (:Update
                      (Transformation|SetRelativeLocation (Variables|Default|GetBox_Collision) (Math|Vector|Lerp(Vector) "0, 0,4.000000" "0, 0, 0" _alpha_2) false false))
                    (:Finished
                      (Rendering|SetVisibility (Variables|Default|GetPaperSprite_Flower) false false)
                      (Collision|SetActorEnableCollision false)
                      (Game|SpawnActorfromClass "/Game/BluePrint/Object/Spawn/BP_Block_Fix.BP_Block_Fix_C" (Transformation|GetActorTransform) "Undefined" 0 0))))))
            (:then_1
              (bind _alpha_3 (Timeline|Kinoko Play)
                (:Update
                  (Transformation|SetRelativeLocation (Variables|Default|GetPaperSprite_Kinoko) (Math|Vector|Lerp(Vector) "0,-1.000000,6.000000" "0,-1.000000,16.000000" _alpha_3) false false))
                (:Finished
                  (Actor|DestroyActor)
                  (bind _returnvalue (Game|SpawnActorfromClass "/Game/BluePrint/Object/BP_PickUp_Kinoko.BP_PickUp_Kinoko_C" (Math|Transform|MakeTransform (+ "0, 0,16.000000" (Transformation|GetActorLocation))) "Undefined" 0 0))
                  (Pawn|SpawnDefaultController _returnvalue))))))
        (:NewEnumerator1
          ;[1 1 1] Flower
          (Utilities|FlowControl|Sequence :!label _label
            (:then_0
              (bind _alpha_4 (Timeline|BlockUp2 Play)
                (:Update
                  (Transformation|SetRelativeLocation (Variables|Default|GetBox_Collision) (Math|Vector|Lerp(Vector) "0, 0, 0" "0, 0,4.000000" _alpha_4) false false))
                (:Finished
                  (bind _alpha_5 (Timeline|BlockDown2 Play)
                    (:Update
                      (Transformation|SetRelativeLocation (Variables|Default|GetBox_Collision) (Math|Vector|Lerp(Vector) "0, 0,4.000000" "0, 0, 0" _alpha_5) false false))
                    (:Finished
                      (Rendering|SetVisibility (Variables|Default|Get31_Block_hatena) false false)
                      (Collision|SetActorEnableCollision false)
                      (Game|SpawnActorfromClass "/Game/BluePrint/Object/Spawn/BP_Block_Fix.BP_Block_Fix_C" (Transformation|GetActorTransform) "Undefined" 0 0))))))
            (:then_1
              (bind _alpha_6 (Timeline|Kinoko2 Play)
                (:Update
                  (Transformation|SetRelativeLocation (Variables|Default|GetPaperSprite_Flower) (Math|Vector|Lerp(Vector) "0,-1.000000,6.000000" "0,-1.000000,16.000000" _alpha_6) false false))
                (:Finished
                  (Actor|DestroyActor)
                  (Game|SpawnActorfromClass "/Game/BluePrint/Object/BP_PickUp_Flower.BP_PickUp_Flower_C" (Math|Transform|MakeTransform (+ "0, 0,16.000000" (Transformation|GetActorLocation))) "Undefined" 0 0))))))
        (:NewEnumerator2
          (goto _label))))))

(event OnComponentBeginOverlap(Box_Top)
  (params (OverlappedComponent :type Primitive%20Component%20Object%20Reference) (OtherActor :type Actor%20Object%20Reference) (OtherComp :type Primitive%20Component%20Object%20Reference) (OtherBodyIndex :type Integer) (bFromSweep :type Boolean) (SweepResult :type Hit%20Result%20Structure%20%28by%20ref%29))
  (Utilities|Launch OtherActor
    (:CastFailed
      (Game|Damage|ApplyDamage OtherActor 1.0 0 0))))

(event EventBeginPlay
  (Collision|SetCollisionEnabled (Variables|Default|GetBox_Top) "NoCollision"))

(event Collision|EventActorBeginOverlap
  (params (OtherActor :type Actor%20Object%20Reference)))

(event EventTick
  (params (DeltaSeconds :type Float%20%28single-precision%29)))

(fn ConstructionScript)