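; 1UP pickup that walks along on its own and grants an extra life when collected.
; Tick feeds constant forward movement input, and a forward box overlap turns it around, briefly disabling that box's collision to debounce the flip.
; Overlapping BP_Start calls PickUp1Up on the game instance, plays a sound, spawns a 1UP text actor just above it and destroys the pickup.
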(event OnComponentBeginOverlap(Box_Forward)
  (params (OverlappedComponent :type Primitive%20Component%20Object%20Reference) (OtherActor :type Actor%20Object%20Reference) (OtherComp :type Primitive%20Component%20Object%20Reference) (OtherBodyIndex :type Integer) (bFromSweep :type Boolean) (SweepResult :type Hit%20Result%20Structure%20%28by%20ref%29))
  ;[1 1 1] 碰撞调头
  (Transformation|SetActorRotation (Math|Rotator|CombineRotators "0,180.000000, 0" (Transformation|GetActorRotation)))
  (Collision|SetCollisionEnabled (Variables|Default|GetBox_Forward) "NoCollision")
  (Utilities|FlowControl|Delay 0.2)
  (Collision|SetCollisionEnabled (Variables|Default|GetBox_Forward) "QueryOnly"))

(event EventBeginPlay)

(event EventTick
  (params (DeltaSeconds :type Float%20%28single-precision%29))
  ;[1 1 1] 移动
  (Pawn|Input|AddMovementInput (Transformation|GetActorForwardVector) 1.0 false))

(event Collision|EventActorBeginOverlap
  (params (OtherActor :type Actor%20Object%20Reference))
  ;[1 1 1] 获得
  (Utilities|Casting|CastToBP_Start OtherActor)
  (Default|PickUp1Up (.AsBP%20Game%20Instance (Utilities|Casting|CastToBP_GameInstance (Game|GetGameInstance))))
  (Audio|PlaySound2D "/Game/Sound/SE/SE_1up.SE_1up" 1.0 1.0 0.0 0 0)
  (Game|SpawnActorfromClass "/Game/BluePrint/Object/Spawn/BP_Text_1UP.BP_Text_1UP_C" (Math|Transform|MakeTransform (+ (Transformation|GetActorLocation) "0, 0,16.000000")) "Undefined" 0 0)
  (Actor|DestroyActor))

(fn ConstructionScript)