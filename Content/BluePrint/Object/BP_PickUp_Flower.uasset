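; BP_PickUp_Flower is a flower power-up pickup that is collected when a BP_Start actor overlaps it.
; On overlap it tells BP_GameInstance to apply the second power-up and award points, then plays the power-up sound.
; It spawns a BP_Text_1000 score popup slightly above its location and destroys itself.
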(event Collision|EventActorBeginOverlap
  (params (OtherActor :type Actor%20Object%20Reference))
  (bind _returnvalue (Game|GetGameInstance))
  (bind _asbp_game_instance (Utilities|Casting|CastToBP_GameInstance _returnvalue))
  (Utilities|Casting|CastToBP_Start OtherActor)
  (Default|PickUpPowerUp2 _asbp_game_instance)
  (Default|GetPoint _asbp_game_instance 1000)
  (Audio|PlaySound2D "/Game/Sound/SE/SE_PowerUp.SE_PowerUp" 1.0 1.0 0.0 0 0)
  (Game|SpawnActorfromClass "/Game/BluePrint/Object/Spawn/BP_Text_1000.BP_Text_1000_C" (Math|Transform|MakeTransform (+ "0, 0,16.000000" (Transformation|GetActorLocation))) "Undefined" 0 0)
  (Actor|DestroyActor))

(fn ConstructionScript)