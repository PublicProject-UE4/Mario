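; Mario-style question block that yields one coin when the player hits it from below.
; The bottom overlap disables its triggers, awards coin and score through BP_GameInstance, plays a sound and pops a coin upward.
; BlockUp and BlockDown timelines bump the block, which is then replaced by BP_Block_Fix.
; A top trigger, disabled at BeginPlay, calls Launch, whose character-launching cast chain is unwired.
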(event OnComponentBeginOverlap(Box_Bottom)
  (params (OverlappedComponent :type Primitive%20Component%20Object%20Reference) (OtherActor :type Actor%20Object%20Reference) (OtherComp :type Primitive%20Component%20Object%20Reference) (OtherBodyIndex :type Integer) (bFromSweep :type Boolean) (SweepResult :type Hit%20Result%20Structure%20%28by%20ref%29))
  (bind _returnvalue (Game|GetGameInstance))
  (bind _asbp_game_instance (Utilities|Casting|CastToBP_GameInstance _returnvalue))
  (Utilities|Casting|CastToBP_Player OtherActor)
  (Collision|SetCollisionEnabled (Variables|Default|GetBox_Bottom) "NoCollision")
  (Collision|SetCollisionEnabled (Variables|Default|GetBox_Top) "NoCollision")
  (Utilities|FlowControl|DoOnce false
    (:Completed
      (Default|PickUpCoin _asbp_game_instance)
      (Default|GetPoint _asbp_game_instance 200)
      (Audio|PlaySound2D "/Game/Sound/SE/SE_Coin.SE_Coin" 1.0 1.0 0.0 0 0)
      (bind _returnvalue_2 (Game|SpawnActorfromClass "/Game/BluePrint/Object/Spawn/BP_PickUp_Coin_Get.BP_PickUp_Coin_Get_C" (Math|Transform|MakeTransform (+ "0.000000, 0,16.000000" (Transformation|GetActorLocation))) "Undefined" 0 0))
      (Physics|AddImpulse (Variables|/Game/BluePrint/Object/Spawn/BP_PickUp_Coin_Get.BP_PickUp_Coin_Get_C|GetBox _returnvalue_2) "0, 0,300.000000" "None" false)
      (Game|SpawnActorfromClass "/Game/BluePrint/Object/Spawn/BP_Text_200.BP_Text_200_C" (Math|Transform|MakeTransform (+ "0, 0,16.000000" (Transformation|GetActorLocation))) "Undefined" 0 0)
      (bind _alpha (Timeline|Block%20Up Play)
        (:Update
          (Transformation|SetRelativeLocation (Variables|Default|GetBox_Collision) (Math|Vector|Lerp(Vector) "0, 0, 0" "0, 0,4.000000" _alpha) false false))
        (:Finished
          (bind _alpha_2 (Timeline|Block%20Down Play)
            (:Update
              (Transformation|SetRelativeLocation (Variables|Default|GetBox_Collision) (Math|Vector|Lerp(Vector) "0, 0,4.000000" "0, 0, 0" _alpha_2) false false))
            (:Finished
              (Actor|DestroyActor)
              (Game|SpawnActorfromClass "/Game/BluePrint/Object/Spawn/BP_Block_Fix.BP_Block_Fix_C" (Transformation|GetActorTransform) "Undefined" 0 0))))))))

(event OnComponentBeginOverlap(Box_Top)
  (params (OverlappedComponent :type Primitive%20Component%20Object%20Reference) (OtherActor :type Actor%20Object%20Reference) (OtherComp :type Primitive%20Component%20Object%20Reference) (OtherBodyIndex :type Integer) (bFromSweep :type Boolean) (SweepResult :type Hit%20Result%20Structure%20%28by%20ref%29))
  (Utilities|Launch OtherActor
    (:CastFailed
      (Game|Damage|ApplyDamage OtherActor 1.0 0 0))))

(event EventBeginPlay
  (Collision|SetCollisionEnabled (Variables|Default|GetBox_Top) "NoCollision"))

(event Collision|EventActorBeginOverlap
  (params (OtherActor :type Actor%20Object%20Reference)))

(event EventTick
  (params (DeltaSeconds :type Float%20%28single-precision%29)))

(fn ConstructionScript)